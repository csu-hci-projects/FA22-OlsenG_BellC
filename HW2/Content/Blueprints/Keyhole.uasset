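; Keyhole actor that consumes overlapping Key actors and counts each one on a referenced Door.
; After incrementing the Door's key count, it calls the Door's unlock check and destroys the key whatever the result.
; On success, it turns its Plane green, waits briefly, then slides the Plane along relative Y with a timeline, lerping from the current location each update.
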(event `self.ReceiveActorBeginOverlap`
  (params (OtherActor :type "Actor Object Reference"))
  (bind _door (`self.Door`))
  (bind _plane (`self.Plane`))
  (bind (_relativelocation_x _relativelocation_y _relativelocation_z) (`KismetMathLibrary.BreakVector` (`SceneComponent.RelativeLocation` _plane)))
  (bind _askey (cast `/Game/Blueprints/Key` OtherActor))
  (`/Engine/EditorBlueprintResources/StandardMacros.IncrementInt` (`/Game/Blueprints/Door.KeysEntered` _door)
    (:`  `
      (bind _unlocked (`/Game/Blueprints/Door.UnlockCheck` _door))
      (if _unlocked
        (`self.K2_DestroyActor` _askey)
        (`PrimitiveComponent.SetMaterial` (`self.Plane`) 0 "/Game/Materials/DoorGreen.DoorGreen")
        (`KismetSystemLibrary.Delay` 1.5)
        (bind (_direction _opendoor) (`Timeline|Timeline_0`)
          (:`Update`
            (`SceneComponent.K2_SetRelativeLocation` (`self.Plane`) (`KismetMathLibrary.VLerp` (`SceneComponent.RelativeLocation` _plane) (`KismetMathLibrary.MakeVector` _relativelocation_x 197.0 _relativelocation_z) _opendoor) false false)))
        (else
          (`self.K2_DestroyActor` _askey))))))

(fn `UserConstructionScript`)