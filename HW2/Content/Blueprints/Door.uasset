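; A door actor that opens once the number of keys entered matches the number it needs.
; UnlockCheck updates a text render with the remaining key count, triggers OpenDoor on a match and returns the result.
; OpenDoor waits briefly, then a timeline lerps the cube from its current position along relative Y.
; CloseDoor snaps it back instantly to the position saved in the construction script.
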(event `OpenDoor`
  (bind _cube (`self.Cube`))
  (bind (_relativelocation_x _relativelocation_y _relativelocation_z) (`KismetMathLibrary.BreakVector` (`SceneComponent.RelativeLocation` _cube)))
  (`KismetSystemLibrary.Delay` 1.5)
  (bind (_direction _opendoor) (`Timeline|Opening Door`)
    (:`Update`
      (`SceneComponent.K2_SetRelativeLocation` (`self.Cube`) (`KismetMathLibrary.VLerp` (`SceneComponent.RelativeLocation` _cube) (`KismetMathLibrary.MakeVector` _relativelocation_x 197.0 _relativelocation_z) _opendoor) false false))))

(event `CloseDoor`
  (`SceneComponent.K2_SetRelativeLocation` (`self.Cube`) (`self.SpawnPos`) false false))

(fn `UnlockCheck`
  (returns (Unlocked :type Boolean))
  (bind _returnvalue (== (`self.KeysEntered`) (`self.KeysNeeded`)))
  (`TextRenderComponent.K2_SetText` (`self.TextRender`) (`KismetTextLibrary.Conv_IntToText` (- (`self.KeysNeeded`) (`self.KeysEntered`))))
  (if _returnvalue
    (`self.OpenDoor`))
  (return _returnvalue))

(fn `UserConstructionScript`
  (`TextRenderComponent.K2_SetText` (`self.TextRender`) (`KismetTextLibrary.Conv_IntToText` (`self.KeysNeeded`)))
  (set `self.SpawnPos` (`SceneComponent.RelativeLocation` (`self.Cube`))))