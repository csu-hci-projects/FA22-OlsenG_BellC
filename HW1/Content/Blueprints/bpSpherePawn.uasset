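; Player pawn for a physics rolling-ball game, with mouse look, jumping, a hold-to-brake action, pause menu and HUD.
; Movement applies camera-relative torque to the sphere mesh; any hit re-arms the impulse jump, and a gate zeroes velocities while braking.
; Construction sets health from RollingGameMode difficulty.
; On destruction it removes the HUD, then notifies the game mode if lives remain or shows the Game Over widget.
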(event `InputAxis|Turn Right / Left Mouse`
  (params (AxisValue :type "Float (single-precision)"))
  ;[1 1 1] Camera Control - Mouse
  (`self.AddControllerYawInput` AxisValue))

(event `InputAxis|Look Up / Down Mouse`
  (params (AxisValue :type "Float (single-precision)"))
  ;[1 1 1] Camera Control - Mouse
  (`self.AddControllerPitchInput` AxisValue))

(event `InputAxis|MoveLeftRightPrimary`
  (params (AxisValue :type "Float (single-precision)"))
  ;[1 1 1] Move X Y Axis Primary
  (`PrimitiveComponent.AddTorqueInDegrees` (`self.StaticMeshSphere`) (* (* (`KismetMathLibrary.GetForwardVector` (`KismetMathLibrary.MakeRotator` 0.0 0.0 (.yaw (`self.GetControlRotation`)))) (`self.TorqueValue`)) AxisValue) "None" true))

(event `InputAction|Jump`
  (params (Key :type "Key Structure"))
  ;[1 1 1] Jump (and plays sound)
  (:`Pressed`
    (if (`self.CanBallJump`)
      (`PrimitiveComponent.AddImpulse` (`self.StaticMeshSphere`) (`KismetMathLibrary.MakeVector` 0.0 0.0 (`self.Impulse`)) "None" true)
      (set `self.CanBallJump` false)
      (`GameplayStatics.PlaySound2D` "/Game/RetroSoundEffects1/Cues/Jump_1_Cue.Jump_1_Cue" 1.0 1.0 0.0 null null false))))

(event `InputAxis|MoveForwardBackPrimary`
  (params (AxisValue :type "Float (single-precision)"))
  ;[1 1 1] Move X Y Axis Primary
  (`PrimitiveComponent.AddTorqueInDegrees` (`self.StaticMeshSphere`) (* (* (`KismetMathLibrary.GetRightVector` (`self.GetControlRotation`)) (`self.TorqueValue`)) AxisValue) "None" true))

(event `InputAxis|MoveLeftRightSecondary`
  (params (AxisValue :type "Float (single-precision)"))
  ;[1 1 1] Move X Y Axis Secondary
  (`PrimitiveComponent.AddTorqueInDegrees` (`self.StaticMeshSphere`) (* (* (`KismetMathLibrary.GetForwardVector` (`KismetMathLibrary.MakeRotator` 0.0 0.0 (.yaw (`self.GetControlRotation`)))) (`self.TorqueValue`)) AxisValue) "None" true))

(event `self.ReceiveHit`
  (params (MyComp :type "PrimitiveComponent Object Reference") (Other :type "Actor Object Reference") (OtherComp :type "PrimitiveComponent Object Reference") (bSelfMoved :type Boolean) (HitLocation :type "Vector Structure") (HitNormal :type "Vector Structure") (NormalImpulse :type "Vector Structure") (Hit :type "HitResult Structure (by ref)"))
  ;[1 1 1] Event Hit (Ball hits ground, enables jump, and plays sound when is false but still enables jump)
  (if (not (`self.CanBallJump`))
    (`GameplayStatics.PlaySound2D` "/Game/Retro_8Bit_Sounds/Impacts/Cues/retro_impact_hit_11_Cue.retro_impact_hit_11_Cue" 1.0 1.0 0.0 null null false))
  (set `self.CanBallJump` true))

(event `InputAxis|MoveForwardBackSecondary`
  (params (AxisValue :type "Float (single-precision)"))
  ;[1 1 1] Move X Y Axis Secondary
  (`PrimitiveComponent.AddTorqueInDegrees` (`self.StaticMeshSphere`) (* (* (`KismetMathLibrary.GetRightVector` (`self.GetControlRotation`)) (`self.TorqueValue`)) AxisValue) "None" true))

(event `self.ReceiveDestroyed`
  (bind _returnvalue (`GameplayStatics.GetPlayerController` 0))
  (bind _hudref (`self.HUDref`))
  ;[1 1 1] Respawn
  (`/Engine/EditorBlueprintResources/StandardMacros.IsValid` _hudref
    (:`Is Valid`
      (`Widget.RemoveFromParent` _hudref))
    (:`Is Not Valid`
      _))
  (bind _asrolling_game_mode (cast `/Game/Blueprints/RollingGameMode` (`GameplayStatics.GetGameMode`)))
  (if (> (`/Game/Blueprints/RollingGameMode.Lives` _asrolling_game_mode) 0)
    (`/Game/Blueprints/RollingGameMode.OnPlayerDied` _asrolling_game_mode)
    (else
      (`/Engine/EditorBlueprintResources/StandardMacros.IncrementInt` (`/Game/Blueprints/RollingGameMode.GameOvers` _asrolling_game_mode)
        (:`  `
          (bind _returnvalue_2 (`|CreateWidget` "/Game/UI/GameOver.GameOver_C" _returnvalue))
          (`UserWidget.AddToViewport` _returnvalue_2 0)
          (`WidgetBlueprintLibrary.SetInputMode_UIOnlyEx` _returnvalue _returnvalue_2)
          (set `PlayerController.bShowMouseCursor` true _returnvalue))))))

(event `InputAxis|StopRolling`
  (params (AxisValue :type "Float (single-precision)"))
  (bind _staticmeshsphere (`self.StaticMeshSphere`))
  ;[1 1 1] Stop Rolling on LShift press/hold
  (`/Engine/EditorBlueprintResources/StandardMacros.Gate` true :!label _label
    (:`Exit`
      (`PrimitiveComponent.SetPhysicsLinearVelocity` _staticmeshsphere (0.0 0.0 0.0) false "None")
      (`PrimitiveComponent.SetPhysicsAngularVelocityInDegrees` _staticmeshsphere (0.0 0.0 0.0) false "None"))))

(event `InputAction|StopRolling`
  (params (Key :type "Key Structure"))
  ;[1 1 1] Stop Rolling on LShift press/hold
  (:`Pressed`
    (goto _label :!via `Open`))
  (:`Released`
    (goto _label :!via `Close`)))

(event `InputAction|Pause` :paused true
  (params (Key :type "Key Structure"))
  (bind _returnvalue (`GameplayStatics.GetPlayerController` 0))
  (bind _returnvalue_2 (`GameplayStatics.GetPlayerController` 0))
  ;[1 1 1] Pause
  (:`Pressed`
    (`/Engine/EditorBlueprintResources/StandardMacros.FlipFlop`
      (:`A`
        (`/Engine/EditorBlueprintResources/StandardMacros.IsValid` (`self.PauseRef`)
          (:`Is Valid`
            _)
          (:`Is Not Valid`
            (bind _returnvalue_3 (`|CreateWidget` "/Game/UI/Pause_Menu.Pause_Menu_C" (`GameplayStatics.GetPlayerController` 0)))
            (bind _output_get (set `self.PauseRef` _returnvalue_3))))
        (`UserWidget.AddToViewport` _output_get 0)
        (`GameplayStatics.SetGamePaused` true)
        (`WidgetBlueprintLibrary.SetInputMode_GameAndUIEx` _returnvalue null)
        (set `PlayerController.bShowMouseCursor` true _returnvalue))
      (:`B`
        (`Widget.RemoveFromParent` (`self.PauseRef`))
        (`WidgetBlueprintLibrary.SetInputMode_GameOnly` _returnvalue_2)
        (set `PlayerController.bShowMouseCursor` false _returnvalue_2)
        (`GameplayStatics.SetGamePaused` false)))))

(event `self.ReceiveBeginPlay`
  ;[1 1 1] HUD Display
  (bind _returnvalue (`GameplayStatics.GetCurrentLevelName` true))
  (if (not (== _returnvalue "Main_Menu"))
    (`/Engine/EditorBlueprintResources/StandardMacros.IsValid` (`self.HUDref`)
      (:`Is Not Valid`
        (bind _returnvalue_2 (`|CreateWidget` "/Game/UI/HUD_Display.HUD_Display_C" (`GameplayStatics.GetPlayerController` 0)))
        (bind _output_get (set `self.HUDref` _returnvalue_2))
        (`UserWidget.AddToViewport` _output_get 0)))))

(fn `UserConstructionScript`
  (bind _asrolling_game_mode (cast `/Game/Blueprints/RollingGameMode` (`GameplayStatics.GetGameMode`)))
  (switch `/Game/Blueprints/Difficulties` (`/Game/Blueprints/RollingGameMode.Difficulty` _asrolling_game_mode)
    (:`NewEnumerator0`
      (bind _output_get (set `self.MaxHealth` 8))
      (set `self.Health` _output_get))
    (:`NewEnumerator1`
      (bind _output_get_2 (set `self.MaxHealth` 4))
      (set `self.Health` _output_get_2))
    (:`NewEnumerator2`
      (bind _output_get_3 (set `self.MaxHealth` 2))
      (set `self.Health` _output_get_3))))