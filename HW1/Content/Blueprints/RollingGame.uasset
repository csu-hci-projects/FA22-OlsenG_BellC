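; RollingGame handles saving and loading of player progress for a rolling game.
; SaveGame creates a RollingSaveGame object, copies in the continue flag, score, high score, difficulty and current level, then writes it to a single fixed slot.
; LoadGame copies those values back from a save object passed in by the caller, without reading the slot itself.
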(fn `LoadGame`
  (params (GameSave :type "/Game/Blueprints/RollingSaveGame Object Reference"))
  (set `self.Score` (`/Game/Blueprints/RollingSaveGame.Score` GameSave))
  (set `self.HighScore` (`/Game/Blueprints/RollingSaveGame.HighScore` GameSave))
  (set `self.CurrentLevel` (`/Game/Blueprints/RollingSaveGame.Level` GameSave))
  (set `self.Difficulty` (`/Game/Blueprints/RollingSaveGame.Difficulty` GameSave))
  (set `self.CanContinue` (`/Game/Blueprints/RollingSaveGame.Continue` GameSave)))

(fn `SaveGame`
  (params (CanContinue :type Boolean))
  (bind _output_get (set `self.CanContinue` CanContinue))
  (bind _returnvalue (`GameplayStatics.CreateSaveGameObject` "/Game/Blueprints/RollingSaveGame.RollingSaveGame_C"))
  (set `/Game/Blueprints/RollingSaveGame.Continue` _output_get _returnvalue)
  (set `/Game/Blueprints/RollingSaveGame.Score` (`self.Score`) _returnvalue)
  (set `/Game/Blueprints/RollingSaveGame.HighScore` (`self.HighScore`) _returnvalue)
  (set `/Game/Blueprints/RollingSaveGame.Difficulty` (`self.Difficulty`) _returnvalue)
  (set `/Game/Blueprints/RollingSaveGame.Level` (`self.CurrentLevel`) _returnvalue)
  (`GameplayStatics.SaveGameToSlot` _returnvalue "SavedGame"))