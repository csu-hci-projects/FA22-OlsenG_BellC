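; Coin pickup Blueprint for a rolling-ball game that adds points to the score when the player's sphere pawn collects it.
; On BeginPlay it reads the difficulty from RollingGameMode and sets its point value, higher on harder settings.
; On overlap with bpSpherePawn it passes those points to the game mode's UpdateScore, plays a 2D pickup sound and destroys itself.
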(event `self.ReceiveBeginPlay`
  (bind _asrolling_game_mode (cast `/Game/Blueprints/RollingGameMode` (`GameplayStatics.GetGameMode`)))
  (switch `/Game/Blueprints/Difficulties` (`/Game/Blueprints/RollingGameMode.Difficulty` _asrolling_game_mode)
    (:`NewEnumerator0`
      (set `self.Points` 5))
    (:`NewEnumerator1`
      (set `self.Points` 10))
    (:`NewEnumerator2`
      (set `self.Points` 15))))

(event `self.ReceiveActorBeginOverlap`
  (params (OtherActor :type "Actor Object Reference"))
  (cast `/Game/Blueprints/bpSpherePawn` OtherActor)
  (bind _asrolling_game_mode (cast `/Game/Blueprints/RollingGameMode` (`GameplayStatics.GetGameMode`)))
  (`/Game/Blueprints/RollingGameMode.UpdateScore` _asrolling_game_mode (`self.Points`))
  (`GameplayStatics.PlaySound2D` "/Game/Retro_8Bit_Sounds/Collectables/Wavs/retro_collect_pickup_coin_10.retro_collect_pickup_coin_10" 1.0 1.0 0.0 null null)
  (`self.K2_DestroyActor`))

(fn `UserConstructionScript`)