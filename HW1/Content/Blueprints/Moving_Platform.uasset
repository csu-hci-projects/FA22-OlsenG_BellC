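; Moving platform actor that shuttles back and forth in the level.
; Tick offsets the actor along the normalized Direction, scaled by Speed and delta seconds, without sweeping.
; A looping timer started on BeginPlay fires Change_Direction every TimeToChange seconds, negating Direction's Y and zeroing X and Z, so movement after the first reversal is confined to the Y axis.
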(event `self.ReceiveTick`
  (params (DeltaSeconds :type "Float (single-precision)"))
  ;[1 1 1] For every frame, update location
  (`self.K2_AddActorWorldOffset` (* (`KismetMathLibrary.Normal` (`self.Direction`)) (* (`self.Speed`) (`GameplayStatics.GetWorldDeltaSeconds`)))))

(event `self.ReceiveBeginPlay`
  ;[1 1 1] Timer that runs changed direction periodically
  (`KismetSystemLibrary.K2_SetTimerDelegate` (delegate `Change_Direction`) (`self.TimeToChange`) true))

(event `Change_Direction`
  ;[1 1 1] Timer that runs changed direction periodically
  (set `self.Direction` (* (`self.Direction`) (0.0 -1.0 0.0))))

(fn `UserConstructionScript`)